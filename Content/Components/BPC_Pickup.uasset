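; Pickup component that lets BP_TestCharacter see an interact prompt on the owning actor and pick it up into an inventory.
; Start and stop interact events track the interactor and set or clear the TextRenderer prompt, which Tick rotates toward that character's camera.
; Interact prints a pickup message, passes ItemData to the interactor's BPC_Inventory, and destroys the owning actor if the add succeeds.
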(event `/Game/Components/BPI_Interactable.StopShowInteract`
  (params (Interactor :type "Actor Object Reference"))
  (`self.Interactor`
    (:`then`
      (bind _textrenderer (`self.TextRenderer`)
        (:`then`
          (`TextRenderComponent.K2_SetText` _textrenderer (`|FormatText` ""))
          (set `self.Interactor` null))
        (:`else`)))
    (:`else`)))

(event `/Game/Components/BPI_Interactable.StartShowInteract`
  (params (Interactor :type "Actor Object Reference"))
  (`/Engine/EditorBlueprintResources/StandardMacros.IsValid` (`self.TextRenderer`)
    (:`Is Valid`
      (bind _asbp_test_character (cast `/Game/BP_TestCharacter` Interactor))
      (set `self.Interactor` _asbp_test_character)
      (`TextRenderComponent.K2_SetText` (`self.TextRenderer`) (`|FormatText` "Press [E] to pickup.")))))

(event `/Game/Components/BPI_Interactable.Interact`
  (params (Interactor :type "Actor Object Reference"))
  (bind _returnvalue (`Actor.GetComponentByClass` Interactor "/Game/Components/BPC_Inventory.BPC_Inventory_C"))
  (`KismetSystemLibrary.PrintString` (`KismetTextLibrary.Conv_TextToString` (`|FormatText` "Pickup {name}." (`KismetSystemLibrary.GetObjectName` (`self.GetOwner`)))))
  (`/Engine/EditorBlueprintResources/StandardMacros.IsValid` _returnvalue
    (:`Is Valid`
      (bind _success (`/Game/Components/BPC_Inventory.AddItem` _returnvalue (`self.ItemData`)))
      (if _success
        (`Actor.K2_DestroyActor` (`self.GetOwner`))))))

(event `self.ReceiveTick`
  (params (DeltaSeconds :type "Float (single-precision)"))
  (`self.TextRenderer`
    (:`then`
      (bind _interactor (`self.Interactor`)
        (:`then`
          (`SceneComponent.K2_SetWorldRotation` (`self.TextRenderer`) (`KismetMathLibrary.FindLookAtRotation` (`SceneComponent.K2_GetComponentLocation` (`self.TextRenderer`)) (`SceneComponent.K2_GetComponentLocation` (`/Game/BP_TestCharacter.Camera` _interactor))) false false))
        (:`else`)))
    (:`else`)))