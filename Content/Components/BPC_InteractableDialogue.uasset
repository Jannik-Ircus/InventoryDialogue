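; BPC_InteractableDialogue is a component that shows an interaction prompt for starting dialogue.
; Preview start stores the BP_TestCharacter interactor and sets the TextRenderer prompt, while preview stop clears both.
; Each tick, the text rotates to face the interactor's camera.
; Start, stop and interact events each invoke a matching On-event call, with no dialogue logic in this graph.
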(event `/Game/Components/BPI_Interactable.StopShowInteract`
  (params (Interactor :type "Actor Object Reference"))
  (`self.OnStopPreviewInteraction`)
  (`self.Interactor`
    (:`then`
      (bind _text_renderer (`self.Text Renderer`)
        (:`then`
          (`TextRenderComponent.K2_SetText` _text_renderer (`|FormatText` ""))
          (set `self.Interactor` null))
        (:`else`)))
    (:`else`)))

(event `/Game/Components/BPI_Interactable.StartShowInteract`
  (params (Interactor :type "Actor Object Reference"))
  (`self.OnStartPreviewInteraction`)
  (`/Engine/EditorBlueprintResources/StandardMacros.IsValid` (`self.Text Renderer`)
    (:`Is Valid`
      (bind _asbp_test_character (cast `/Game/BP_TestCharacter` Interactor))
      (set `self.Interactor` _asbp_test_character)
      (`TextRenderComponent.K2_SetText` (`self.Text Renderer`) (`|FormatText` "Press [E] to start dialogue.")))))

(event `/Game/Components/BPI_Interactable.Interact`
  (params (Interactor :type "Actor Object Reference"))
  (`self.OnInteract`))

(event `self.ReceiveTick`
  (params (DeltaSeconds :type "Float (single-precision)"))
  (`self.Text Renderer`
    (:`then`
      (bind _interactor (`self.Interactor`)
        (:`then`
          (`SceneComponent.K2_SetWorldRotation` (`self.Text Renderer`) (`KismetMathLibrary.FindLookAtRotation` (`SceneComponent.K2_GetComponentLocation` (`self.Text Renderer`)) (`SceneComponent.K2_GetComponentLocation` (`/Game/BP_TestCharacter.Camera` _interactor))) false false))
        (:`else`)))
    (:`else`)))