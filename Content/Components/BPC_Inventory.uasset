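; Inventory component that stores items in a slot array, filled to MaxSize at BeginPlay, when it also spawns a BP_ItemPreviewer high above the world origin.
; AddItem increments the quantity of a matching ID, otherwise fills the first empty-ID slot or reports a full inventory.
; RemoveItem decrements the quantity, removing the array element outright at the last one.
; SwapItems exchanges two slots by index.
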(event `self.ReceiveBeginPlay`
  (`|ExecutionSequence`
    (:`then_0`
      (for _ (range (`self.MaxSize`))
        (`KismetArrayLibrary.Array_Add` (`self.Inventory`))))
    (:`then_1`
      (`|SpawnActorFromClass` "/Game/Blueprints/BP_ItemPreviewer.BP_ItemPreviewer_C" (`KismetMathLibrary.MakeTransform` (0.0 0.0 5000.0)) "Undefined" "MultiplyWithRoot" null null))))

(fn `AddItem`
  (params (Item :type "/Game/Structs/InventoryItem Structure"))
  (returns (Success :type Boolean))
  (for (_array_element _array_index) (`self.Inventory`)
    (bind (_id _itemname _icon _quantity) (break `/Game/Structs/InventoryItem` _array_element))
    (if (`KismetStringLibrary.EqualEqual_StrStr` _id (`.ID_6_59D739994CC9FFF9A48EE785840BC17C` (break `/Game/Structs/InventoryItem` Item)))
      (bind _structout (setmembers `/Game/Structs/InventoryItem` :`StructRef` _array_element :`Quantity` (+ _quantity 1)))
      (`KismetArrayLibrary.Array_Set` (`self.Inventory`) _array_index _structout)
      (return true)))
  (for (_array_element_2 _array_index_2) (`self.Inventory`)
    (if (`KismetStringLibrary.EqualEqual_StrStr` (`.ID_6_59D739994CC9FFF9A48EE785840BC17C` (break `/Game/Structs/InventoryItem` _array_element_2)))
      (`KismetArrayLibrary.Array_Set` (`self.Inventory`) _array_index_2 Item)
      (return true)))
  (`KismetSystemLibrary.PrintString` "Inventory full" true true (struct :`R` 1.0 :`A` 1.0))
  (return false))

(fn `RemoveItem`
  (params (Item :type "/Game/Structs/InventoryItem Structure"))
  (returns (Success :type Boolean))
  (for (_array_element _array_index) (`self.Inventory`)
    (bind (_id _itemname _icon _quantity) (break `/Game/Structs/InventoryItem` _array_element))
    (if (`KismetStringLibrary.EqualEqual_StrStr` _id (`.ID_6_59D739994CC9FFF9A48EE785840BC17C` (break `/Game/Structs/InventoryItem` Item)))
      (if (> _quantity 1)
        (bind _structout (setmembers `/Game/Structs/InventoryItem` :`StructRef` _array_element :`Quantity` (- _quantity 1)))
        (`KismetArrayLibrary.Array_Set` (`self.Inventory`) _array_index _structout)
        (return true)
        (else
          (`KismetArrayLibrary.Array_RemoveItem` (`self.Inventory`) _array_element)
          (return true)))))
  (return false))

(fn `SwapItems`
  (params (SourceIndex :type Integer) (TargetIndex :type Integer))
  (locals (TempItem :type "/Game/Structs/InventoryItem Structure") (Source :type Integer) (Target :type Integer))
  (set `local.Source` SourceIndex)
  (set `local.Target` TargetIndex)
  (if (and (>= (`self.MaxSize`) (`local.Source`)) (>= (`self.MaxSize`) (`local.Target`)))
    (set `local.TempItem` (`|GetArrayItem` (`self.Inventory`) (`local.Source`)))
    (`KismetArrayLibrary.Array_Set` (`self.Inventory`) (`local.Source`) (`|GetArrayItem` (`self.Inventory`) (`local.Target`)))
    (`KismetArrayLibrary.Array_Set` (`self.Inventory`) (`local.Target`) (`local.TempItem`))))