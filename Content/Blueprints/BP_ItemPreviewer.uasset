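; BP_ItemPreviewer is an actor that previews an item mesh through a scene capture.
; Its construction script adds itself to the SceneCaptureComponent2D show-only list.
; SetMesh swaps the static mesh and scales it uniformly from its Z bounds extent, normalizing previewed items to the same height.
; MoveObject turns a 2D delta into spring arm yaw and a clamped arm length for orbit and zoom.
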(fn `MoveObject`
  (params (Delta :type "Vector2D Structure"))
  (bind (_x _y) (`KismetMathLibrary.BreakVector2D` Delta))
  (`SceneComponent.K2_AddWorldRotation` (`self.SpringArm`) (`KismetMathLibrary.MakeRotator` 0.0 0.0 (* _x 0.3)) false false)
  (set `SpringArmComponent.TargetArmLength` (`KismetMathLibrary.FClamp` (+ (* _y 0.3) (`SpringArmComponent.TargetArmLength` (`self.SpringArm`))) 100.0 250.0) (`self.SpringArm`)))

(fn `SetMesh`
  (params (NewMesh :type "StaticMesh Object Reference"))
  (bind (_returnvalue_x _returnvalue_y _returnvalue_z) (`KismetMathLibrary.BreakVector` (/ 50 (`.BoxExtent` (`KismetMathLibrary.BreakBoxSphereBounds` (`StaticMesh.GetBounds` NewMesh))))))
  (`StaticMeshComponent.SetStaticMesh` (`self.StaticMesh`) NewMesh)
  (`SceneComponent.SetWorldScale3D` (`self.StaticMesh`) (`KismetMathLibrary.Conv_DoubleToVector` _returnvalue_z)))

(fn `UserConstructionScript`
  (`KismetArrayLibrary.Array_Add` (`SceneCaptureComponent.ShowOnlyActors` (`self.SceneCaptureComponent2D`)) self))